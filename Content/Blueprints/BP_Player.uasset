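; Player character for a multiplayer game where humans drop poop actors and kick them, with Enhanced Input for movement, camera and sprint.
; Pooping, kicking and sprinting use server-to-client event chains, with montages setting an AnimBusy flag that blocks movement.
; Kicking turns the body toward control yaw on a timeline, then line-traces for BP_Poop to launch.
; Sprinting drains PoopMeter to raise walk speed and feeds it to the HUD.
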(event Custom|PlayKickMontageToServer
  ;[0 0 0] Kick
  ;;[0 0 0] Client / Server
  (CallFunction|PlayKickMontagetoClients)
  (CallFunction|TurnPlayer&Kick))

(event Custom|PlayKickMontageToClients
  ;[0 0 0] Kick
  ;;[0 0 0] Logic
  (if (not (Variables|Default|GetAnimBusy))
    (Animation|Montage|PlayMontage (Variables|Character|GetMesh) "/Game/Animations/HoomanAnimKick_Anim_Montage.HoomanAnimKick_Anim_Montage"
      (:then
        (Variables|Default|SetAnimBusy true))
      (:OnCompleted
        (Variables|Default|SetAnimBusy false)))))

(event Custom|SprintOnClients
  (params (canSprintOnClient :type Boolean))
  (bind _charactermovement (Variables|Character|GetCharacterMovement))
  ;[0 0 0] Sprinting
  ;;[0 0 0] Logic
  (if (and canSprintOnClient (> (Variables|Default|GetPoopMeter) 0.0))
    (Variables|Default|SetPoopMeter (- (Variables|Default|GetPoopMeter) (Variables|Default|GetPoopRunReduce)))
    (Variables|/Script/Engine.CharacterMovementComponent|SetMaxWalkSpeed _charactermovement 7.5e+02)
    (else
      (Variables|/Script/Engine.CharacterMovementComponent|SetMaxWalkSpeed _charactermovement 3e+02))))

(event Custom|SprintOnServer
  (params (canSprintOnServer :type Boolean))
  ;[0 0 0] Sprinting
  ;;[0 0 0] Server / Client
  (CallFunction|SprintonClients canSprintOnServer))

(event Custom|TurnPlayer&Kick
  ;[0 0 0] Kick
  ;;[0 0 0] TurnPlayer
  (if (> (Variables|Default|GetSettings) 0)
    (Variables|Default|SetStartRotation (Transformation|GetActorRotation))
    (bind _turntrack (Timeline|Timeline PlayFromStart)
      (:Update
        (Transformation|SetActorRotation (Math|Rotator|Lerp(Rotator) (Variables|Default|GetStartRotation) (Math|Rotator|MakeRotator (.roll (Variables|Default|GetStartRotation)) (.pitch (Variables|Default|GetStartRotation)) (.yaw (Pawn|GetControlRotation :!class /Script/Engine.Pawn))) _turntrack true)))
      (:Finished
        (CallFunction|KICK)))))

(event Custom|KICK
  ;[0 0 0] Kick
  ;;[0 0 0] Kick The Poop
  (bind (_outhit _returnvalue) (Collision|LineTraceByChannel (Transformation|GetWorldLocation (Variables|Character|GetMesh)) (Transformation|GetWorldLocation (Variables|Default|GetTraceStartPoint)) "TraceTypeQuery2" false 0 "ForDuration"))
  (if (and _returnvalue (== (Utilities|GetClass (.HitActor (Collision|BreakHitResult _outhit))) "/Game/Blueprints/Props/BP_Poop.BP_Poop_C"))
    (Class|BIPoop|KickPoop(Message) (.HitActor (Collision|BreakHitResult _outhit)) (Variables|Default|GetKickForce))))

(event Custom|PoopSpawnInServer
  (CallFunction|MontagestoClients)
  (Game|SpawnActorfromClass "/Game/Blueprints/Props/BP_Poop.BP_Poop_C" (Math|Transform|MakeTransform (Transformation|GetWorldLocation (Variables|Default|GetPoopSpawn)) "0, 0, 0" "1.000000,1.000000,1.000000") "Undefined" "MultiplyWithRoot" 0 0))

(event Custom|MontagesToClients
  (if (not (Variables|Default|GetAnimBusy))
    (Animation|Montage|PlayMontage (Variables|Character|GetMesh) "/Game/Animations/AM_HoomanPoop.AM_HoomanPoop"
      (:then
        (Variables|Default|SetAnimBusy true))
      (:OnCompleted
        (Variables|Default|SetAnimBusy false)))))

(event Input|EnhancedActionEvents|EnhancedInputActionIA_Mevement
  (params (ActionValue :type Vector%202D%20Structure) (ElapsedSeconds :type Float%20%28double-precision%29) (TriggeredSeconds :type Float%20%28double-precision%29) (InputAction :type Input%20Action%20Object%20Reference :default "/Game/Inputs/IA_Mevement.IA_Mevement"))
  (bind _returnvalue (Game|GetPlayerController 0))
  (bind _returnvalue_2 (Pawn|GetControlRotation _returnvalue :!class /Script/Engine.Controller))
  ;[0 0 0] Player Input
  (if (not (Variables|Default|GetAnimBusy))
    (Pawn|Input|AddMovementInput (Math|Vector|GetForwardVector (Math|Rotator|MakeRotator 0.0 0.0 (.yaw _returnvalue_2))) (.x ActionValue) false)
    (Pawn|Input|AddMovementInput (Math|Vector|GetRightVector (Math|Rotator|MakeRotator (.roll _returnvalue_2) 0.0 (.yaw _returnvalue_2))) (.y ActionValue) false)))

(event Input|EnhancedActionEvents|EnhancedInputActionIA_CameraMovement
  (params (ActionValue :type Vector%202D%20Structure) (ElapsedSeconds :type Float%20%28double-precision%29) (TriggeredSeconds :type Float%20%28double-precision%29) (InputAction :type Input%20Action%20Object%20Reference :default "/Game/Inputs/IA_CameraMovement.IA_CameraMovement"))
  ;[0 0 0] Camera Movement
  (Pawn|Input|AddControllerYawInput (.x ActionValue))
  (Pawn|Input|AddControllerPitchInput (.y ActionValue)))

(event Input|EnhancedActionEvents|EnhancedInputActionIA_Sprint
  (params (ActionValue :type Boolean) (ElapsedSeconds :type Float%20%28double-precision%29) (TriggeredSeconds :type Float%20%28double-precision%29) (InputAction :type Input%20Action%20Object%20Reference :default "/Game/Inputs/IA_Sprint.IA_Sprint"))
  ;[0 0 0] Sprinting
  ;;[0 0 0] Server / Client
  (:Triggered
    (CallFunction|SprintonServer true)
    (if (> (Variables|/Script/Engine.CharacterMovementComponent|GetMaxWalkSpeed (Variables|Character|GetCharacterMovement)) 3e+02)
      (Variables|/Game/UI/WB_HUD.WB_HUD_C|SetHowMuchPoop (Variables|Default|GetHUD) (Variables|Default|GetPoopMeter))))
  (:Completed
    (CallFunction|SprintonServer false)))

(event Input|EnhancedActionEvents|EnhancedInputActionIA_Kick
  (params (ActionValue :type Boolean) (ElapsedSeconds :type Float%20%28double-precision%29) (TriggeredSeconds :type Float%20%28double-precision%29) (InputAction :type Input%20Action%20Object%20Reference :default "/Game/Inputs/IA_Kick.IA_Kick"))
  ;[0 0 0] Kick
  ;;[0 0 0] Client / Server
  (:Started
    (CallFunction|PlayKickMontagetoServer)
    (CallFunction|TurnPlayer&Kick)))

(event Input|EnhancedActionEvents|EnhancedInputActionIA_Poop
  (params (ActionValue :type Boolean) (ElapsedSeconds :type Float%20%28double-precision%29) (TriggeredSeconds :type Float%20%28double-precision%29) (InputAction :type Input%20Action%20Object%20Reference :default "/Game/Inputs/IA_Poop.IA_Poop"))
  (:Started
    (CallFunction|PoopSpawninServer)))

(event EventBeginPlay
  (bind _returnvalue (Game|GetPlayerController 0))
  ;[0 0 0] Init
  ;;[0 0 0] Input Context
  (bind _asplayer_controller (Utilities|Casting|CastToPlayerController _returnvalue))
  (Utilities|IsValid (PlayerController|LocalPlayerSubsystems|GetEnhancedInputLocalPlayerSubsystem _asplayer_controller)
    (:Is%20Valid
      (Input|AddMappingContext (PlayerController|LocalPlayerSubsystems|GetEnhancedInputLocalPlayerSubsystem _asplayer_controller) "/Game/Inputs/IMC_InputSystem.IMC_InputSystem" 0 "(bIgnoreAllPressedKeysUntilRelease=True,bForceImmediately=False,bNotifyUserSettings=False)")
      (bind _asscreen_hud (Utilities|Casting|CastToScreenHUD (HUD|GetHUD _returnvalue)))
      (Variables|Default|SetHUD (Variables|/Game/UI/ScreenHUD.ScreenHUD_C|GetRef_HUD _asscreen_hud)))))

(fn ConstructionScript)