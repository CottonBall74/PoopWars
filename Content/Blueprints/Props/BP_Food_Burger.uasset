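; Burger food prop that shows a widget when the player pawn enters its collision area and can be consumed.
; The widget is hidden on BeginPlay; the end-overlap event is empty, so it stays visible once shown.
; GetFoodValue returns the burger's FoodValue, and ConsumeFood destroys the actor.
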(event OnComponentBeginOverlap(CollisionArea)
  (params (OverlappedComponent :type Primitive%20Component%20Object%20Reference) (OtherActor :type Actor%20Object%20Reference) (OtherComp :type Primitive%20Component%20Object%20Reference) (OtherBodyIndex :type Integer) (bFromSweep :type Boolean) (SweepResult :type Hit%20Result%20Structure%20%28by%20ref%29))
  (if (== OtherActor (Game|Player|GetPlayerPawn 0))
    (Rendering|SetVisibility (Variables|Default|GetWidget) true false)))

(event OnComponentEndOverlap(CollisionArea)
  (params (OverlappedComponent :type Primitive%20Component%20Object%20Reference) (OtherActor :type Actor%20Object%20Reference) (OtherComp :type Primitive%20Component%20Object%20Reference) (OtherBodyIndex :type Integer)))

(event EventBeginPlay
  (Rendering|SetVisibility (Variables|Default|GetWidget) false false))

(event EventConsumeFood
  (Actor|DestroyActor))

(fn ConstructionScript)

(fn GetFoodValue
  (return (Variables|Default|GetFoodValue)))